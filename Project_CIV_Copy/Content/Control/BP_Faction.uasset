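; BP_Faction tracks a faction's gold, food, wood and metal stockpiles in a turn-based game.
; NextTurn calls NewTurnResourses, which loops over the Owned list and passes each element's Production array to four setters.
; Each setter adds the value at its fixed array index to the running total, so the setters accumulate rather than overwrite.
; NextTurn then calls NewTurnPlaceable, which is an empty stub.
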(fn `newTurnPlaceable`)

(fn `newTurnResourses`
  (for _array_element (`self.Owned`)
    (bind _production (`/Game/Placeable/BP_Placable.production` _array_element))
    (`self.setGold` _production)
    (`self.setFood` _production)
    (`self.setWood` _production)
    (`self.setMetal` _production)))

(fn `nextTurn`
  (`self.newTurnResourses`)
  (`self.newTurnPlaceable`))

(fn `setFood`
  (params (Production :type "Array of Float (double-precision)"))
  (set `self.Food` (+ (`self.Food`) (`|GetArrayItem` Production 1))))

(fn `setGold`
  (params (Production :type "Array of Float (double-precision)"))
  (set `self.Gold` (+ (`self.Gold`) (`|GetArrayItem` Production))))

(fn `setMetal`
  (params (Production :type "Array of Float (double-precision)"))
  (set `self.Metal` (+ (`self.Metal`) (`|GetArrayItem` Production 3))))

(fn `setWood`
  (params (Production :type "Array of Float (double-precision)"))
  (set `self.Wood` (+ (`self.Wood`) (`|GetArrayItem` Production 2))))
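; Player controller for a turn-based hex-tile strategy game, handling camera movement and mouse commands.
; Axis inputs move and rotate the controlled camera pawn, while a toggle blends to a tagged fixed camera and locks movement.
; During an active turn, left click selects the tile under a unit, hex or holding unless an AI faction is current.
; Right click moves the selected unit to reachable tiles and uncovers its visible area.
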(event `InputAxis|ZoomDown`
  (params (AxisValue :type "Float (single-precision)"))
  (if (`self.Movable`)
    (`Pawn.AddMovementInput` (`self.K2_GetPawn`) (`KismetMathLibrary.MakeVector` 0.0 0.0 10.0) AxisValue false)))

(event `InputAxis|Forward`
  (params (AxisValue :type "Float (single-precision)"))
  (bind _returnvalue (`self.K2_GetPawn`))
  (if (`self.Movable`)
    (`Pawn.AddMovementInput` _returnvalue (`self.GetActorForwardVector` _returnvalue) AxisValue false)))

(event `InputAxis|Right`
  (params (AxisValue :type "Float (single-precision)"))
  (bind _returnvalue (`self.K2_GetPawn`))
  (if (`self.Movable`)
    (`Pawn.AddMovementInput` _returnvalue (`self.GetActorRightVector` _returnvalue) AxisValue false)))

(event `InputAxis|TurnUp`
  (params (AxisValue :type "Float (single-precision)"))
  (if (`self.Movable`)
    (bind _asbp_camera (cast `/Game/Control/BP_Camera` (`self.K2_GetPawn`)))
    (`/Game/Control/BP_Camera.camDown` _asbp_camera (* AxisValue (stale `InputAxis|TurnTrue` AxisValue)))))

(event `InputAxis|TurnTrue`
  (params (AxisValue :type "Float (single-precision)"))
  (bind (_sizex _sizey) (`self.GetViewportSize`))
  (bind _output_get (set `self.bShowMouseCursor` (== AxisValue 0.0)))
  (if (not _output_get)
    (`self.SetMouseLocation` (/ _sizex 2) (/ _sizey 2))))

(event `InputAxis|TrurnRight`
  (params (AxisValue :type "Float (single-precision)"))
  (if (`self.Movable`)
    (`Pawn.AddControllerYawInput` (`self.K2_GetPawn`) (* (stale `InputAxis|TurnTrue` AxisValue) AxisValue))))

(event `InputAction|CameraChange`
  (params (Key :type "Key Structure"))
  (:`Pressed`
    (`/Engine/EditorBlueprintResources/StandardMacros.FlipFlop`
      (:`A`
        (bind _outactors (`GameplayStatics.GetAllActorsWithTag` "FixedCamera"))
        (`self.SetViewTargetWithBlend` (`|GetArrayItem` _outactors) 1.0)
        (set `self.Movable` false))
      (:`B`
        (`self.SetViewTargetWithBlend` (`self.K2_GetPawn`) 1.0)
        (set `self.Movable` true)))))

(event `InputAction|LeftClick`
  (params (Key :type "Key Structure"))
  (bind (_bblockinghit _binitialoverlap _time _distance _location _impactpoint _normal _impactnormal _physmat _hitactor) (`GameplayStatics.BreakHitResult` (`self.GetHitResultUnderCursorByChannel` "TraceTypeQuery1")))
  (:`Pressed`
    (bind _isactive (`self.isActiveTurn`))
    (if _isactive
      (bind _asbp_unit (cast `/Game/Placeable/BP_Unit` _hitactor)
        (:`then`
          (`self.select` (`/Game/Placeable/BP_Placable.currentTile` _asbp_unit)))
        (:`CastFailed`
          (bind _asbp_hex_tile (cast `/Game/Hex/BP_HexTile` _hitactor)
            (:`then`
              (`self.select` _asbp_hex_tile))
            (:`CastFailed`
              (bind _asbp_holding (cast `/Game/Placeable/BP_Holding` _hitactor))
              (`self.select` (`/Game/Placeable/BP_Placable.currentTile` _asbp_holding)))))))))

(event `InputAction|RightClick`
  (params (Key :type "Key Structure"))
  (bind (_bblockinghit _binitialoverlap _time _distance _location _impactpoint _normal _impactnormal _physmat _hitactor) (`GameplayStatics.BreakHitResult` (`self.GetHitResultUnderCursorByChannel` "TraceTypeQuery1")))
  (:`Pressed`
    (bind _isactive (`self.isActiveTurn`))
    (if _isactive
      (bind _asbp_hex_tile (cast `/Game/Hex/BP_HexTile` _hitactor)
        (:`then`
          (`self.orderMove` _asbp_hex_tile))
        (:`CastFailed`
          (bind _asbp_unit (cast `/Game/Placeable/BP_Unit` _hitactor)
            (:`then`
              (`self.orderMove` (`/Game/Placeable/BP_Placable.currentTile` _asbp_unit)))
            (:`CastFailed`
              (bind _asbp_holding (cast `/Game/Placeable/BP_Holding` _hitactor))
              (`self.orderMove` (`/Game/Placeable/BP_Placable.currentTile` _asbp_holding)))))))))

(fn `isActiveTurn`
  (returns (isActive :type Boolean))
  (bind _asbp_instance (cast `/Game/Control/BP_Instance` (`GameplayStatics.GetGameInstance`)))
  (return (`/Game/Control/BP_Instance.ActiveTurn` _asbp_instance)))

(fn `orderMove`
  (params (tile :type "/Game/Hex/BP_HexTile Object Reference"))
  (bind _asbp_instance (cast `/Game/Control/BP_Instance` (`GameplayStatics.GetGameInstance`)))
  (bind _selectedunit (`/Game/Control/BP_Instance.SelectedUnit` _asbp_instance))
  (bind _keys (`BlueprintMapLibrary.Map_Keys` (`/Game/Placeable/BP_Unit.reachMap` _selectedunit)))
  (if (`KismetArrayLibrary.Array_Contains` _keys tile)
    (`/Game/Placeable/BP_Unit.navigateTo` _selectedunit tile)
    (`/Game/Placeable/BP_Placable.uncoverVisible` _selectedunit)))

(fn `select`
  (params (tile :type "/Game/Hex/BP_HexTile Object Reference"))
  (bind _asbp_instance (cast `/Game/Control/BP_Instance` (`GameplayStatics.GetGameInstance`)))
  (if (not (`GameplayStatics.ObjectIsA` (`|GetArrayItem` (`/Game/Control/BP_Instance.Factions` _asbp_instance) (`/Game/Control/BP_Instance.factionInd` _asbp_instance)) "/Game/Control/Factions/BPAiFaction.BPAiFaction_C"))
    (`/Game/Control/BP_Instance.select` _asbp_instance tile)))

(fn `UserConstructionScript`)
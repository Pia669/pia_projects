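; Central controller for a turn-based tile strategy game, managing factions, turn order and the current tile and unit selection.
; FactStartLocation spawns a player or AI faction by slot index, gives it a random color and creates its starting holding and unit.
; NextTurn cycles through factions and refreshes the HUD.
; Tile and unit clicks keep both selections in sync, move the reach markers to the selected unit and update the HUD.
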(fn `clickTile`
  (params (tile :type "/Game/Hex/BP_HexTile Object Reference"))
  (`self.updateTile` tile)
  (bind _unit (`/Game/Hex/BP_HexTile.getNextUnit` tile))
  (`self.updateUnit` _unit)
  (`self.updateHUD`))

(fn `clickUnit`
  (params (unit :type "/Game/Placeable/BP_Unit Object Reference"))
  (`self.updateUnit` unit)
  (`self.updateTile` (`/Game/Placeable/BP_Placable.currentTile` unit))
  (`self.updateHUD`))

(fn `factStartLocation`
  (params (tile :type "/Game/Hex/BP_HexTile Object Reference"))
  (bind _colors (`self.colors`))
  (bind _faction (`self.startFaction` tile))
  (`KismetArrayLibrary.Array_Add` (`self.Factions`) _faction)
  (bind _output_get (set `/Game/Control/Factions/BPFaction.Color` (`|GetArrayItem` _colors (`KismetMathLibrary.RandomInteger` (`KismetArrayLibrary.Array_Length` _colors))) _faction))
  (`self.spawnHolding` tile _output_get _faction)
  (`self.spawnUnit` tile _output_get _faction))

(fn `getCurrentPalyerFaction`
  (returns (playerFaction :type "/Game/Control/Factions/BPFaction Object Reference"))
  (if (< (`self.factionInd`) (`self.PLAYER_N_FACTIONS`))
    (return (`|GetArrayItem` (`self.Factions`) (`self.factionInd`)))))

(fn `nextTurn`
  (bind _output_get (set `self.factionInd` (mod (+ (`self.factionInd`) 1) (`self.N_FACTIONS`))))
  (`/Game/Control/Factions/BPFaction.EventStartNewTurn` (`|GetArrayItem` (`self.Factions`) _output_get))
  (`self.updateHUD`))

(fn `spawnHolding`
  (params (tile :type "/Game/Hex/BP_HexTile Object Reference") (color :type "Material Object Reference") (faction :type "/Game/Control/Factions/BPFaction Object Reference"))
  (bind _returnvalue (`|SpawnActorFromClass` "/Game/Placeable/BP_Holding.BP_Holding_C" (`KismetMathLibrary.MakeTransform` (`Actor.K2_GetActorLocation` tile) (struct :`Yaw` 180.0)) "Undefined" "MultiplyWithRoot" null tile color faction null))
  (`/Game/Placeable/BP_Holding.nameHolding` _returnvalue 0)
  (`KismetArrayLibrary.Array_Add` (`/Game/Control/Factions/BPFaction.Owned` faction) _returnvalue))

(fn `spawnUnit`
  (params (tile :type "/Game/Hex/BP_HexTile Object Reference") (color :type "Material Object Reference") (faction :type "/Game/Control/Factions/BPFaction Object Reference"))
  (bind _owned (`/Game/Control/Factions/BPFaction.Owned` faction))
  (bind _returnvalue (`|SpawnActorFromClass` "/Game/Placeable/BP_Unit.BP_Unit_C" (`KismetMathLibrary.MakeTransform` (`Actor.K2_GetActorLocation` tile) (struct :`Yaw` 180.0)) "Undefined" "MultiplyWithRoot" null tile color faction null))
  (`/Game/Placeable/BP_Unit.nameUnit` _returnvalue (`KismetArrayLibrary.Array_Length` _owned))
  (`KismetArrayLibrary.Array_Add` _owned _returnvalue))

(fn `startFaction`
  (params (tile :type "/Game/Hex/BP_HexTile Object Reference"))
  (returns (faction :type "/Game/Control/Factions/BPFaction Object Reference"))
  (bind _returnvalue (`Actor.K2_GetActorLocation` tile))
  (if (< (`KismetArrayLibrary.Array_Length` (`self.Factions`)) (`self.PLAYER_N_FACTIONS`))
    (bind _returnvalue_2 (`|SpawnActorFromClass` "/Game/Control/Factions/BPFaction.BPFaction_C" (`KismetMathLibrary.MakeTransform` (0.0 0.0 0.0)) "Undefined" "MultiplyWithRoot" null _returnvalue null))
    (return _returnvalue_2)
    (else
      (bind _returnvalue_3 (`|SpawnActorFromClass` "/Game/Control/Factions/BPAiFaction.BPAiFaction_C" (`KismetMathLibrary.MakeTransform` (0.0 0.0 0.0)) "Undefined" "MultiplyWithRoot" null _returnvalue null))
      (return _returnvalue_3))))

(fn `updateHUD`
  (bind _foundwidgets (`WidgetBlueprintLibrary.GetAllWidgetsOfClass` "/Game/GUI/HUDWitget.HUDWitget_C"))
  (`/Game/GUI/HUDWitget.Update` (`|GetArrayItem` _foundwidgets)))

(fn `updateTile`
  (params (tile :type "/Game/Hex/BP_HexTile Object Reference"))
  (set `self.SelectedTile` tile))

(fn `updateUnit`
  (params (unit :type "/Game/Placeable/BP_Unit Object Reference"))
  (bind _selectedunit (`self.SelectedUnit`))
  (`/Engine/EditorBlueprintResources/StandardMacros.IsValid` _selectedunit
    (:`Is Valid`
      (`/Game/Placeable/BP_Unit.unmarkRaech` _selectedunit))
    (:`Is Not Valid`
      _))
  (bind _output_get (set `self.SelectedUnit` unit))
  (`/Engine/EditorBlueprintResources/StandardMacros.IsValid` _output_get
    (:`Is Valid`
      (`/Game/Placeable/BP_Unit.markReach` _output_get))))
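; BP_Unit is a turn-based, tile-grid unit that can be selected, moved, made to attack and dismissed, with move points refilled each turn.
; MarkReach has the current tile fill ReachMap with reachable paths; NavigateTo claims the destination immediately and deducts its cost.
; A looping timer interpolates each hop, rising before horizontal travel and descending last.
; On arrival, MoveTo attacks any enemy present, then may re-navigate or refresh non-AI selection.
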(event `self.ReceiveBeginPlay`
  (`parent.ReceiveBeginPlay`)
  (set `self.targetPosition` (`self.K2_GetActorLocation`)))

(event `self.ReceiveTick`
  (params (DeltaSeconds :type "Float (single-precision)"))
  (`parent.ReceiveTick` DeltaSeconds))

(event `EventToMove`
  (bind _returnvalue (`KismetSystemLibrary.K2_SetTimerDelegate` (delegate `EventStep`) 0.01 true)))

(event `EventStep`
  (bind _ret (`self.nearTarget`))
  (if _ret
    (`self.K2_SetActorLocation` (`self.targetPosition`))
    (`KismetSystemLibrary.K2_ClearAndInvalidateTimerHandle` (stale `EventToMove` _returnvalue))
    (`self.moveTo`)
    (else
      (`self.makeStep` (`GameplayStatics.GetWorldDeltaSeconds`)))))

(event `self.EventNewTurn`
  (set `self.movePt` (`self.maxMovePt`)))

(fn `attackEnemy`
  (returns (enemyPresent :type Boolean))
  (bind _finishtile (`self.finishTile`))
  (bind _unit (`/Game/Hex/BP_HexTile.getCurrentUnit` _finishtile))
  (`/Engine/EditorBlueprintResources/StandardMacros.IsValid` _unit
    (:`Is Valid`
      (bind _survive (`self.attacked` _unit self))
      (return (or (> (`KismetArrayLibrary.Array_Length` (`/Game/Hex/BP_HexTile.Units` (`self.currentTile`))) 0) _survive)))
    (:`Is Not Valid`
      (bind _survive_2 (`self.attacked` (`/Game/Hex/BP_HexTile.holding` _finishtile) self))
      (return _survive_2))))

(fn `choosePosition`
  (bind (_returnvalue_x _returnvalue_y _returnvalue_z) (`KismetMathLibrary.BreakVector` (`self.K2_GetActorLocation`)))
  (bind (_returnvalue_x_2 _returnvalue_y_2 _returnvalue_z_2) (`KismetMathLibrary.BreakVector` (`self.K2_GetActorLocation` (`self.tragetTile`))))
  (bind _value (`BlueprintMapLibrary.Map_Find` (`self.reachMap`) (`self.finishTile`)))
  (if (== (`self.K2_GetActorLocation`) (`self.K2_GetActorLocation` (`self.tragetTile`)))
    (if (`/Game/Control/BP_Path.attacked` _value)
      (bind _tile (`/Game/Control/BP_Path.getCurrent` _value))
      (set `self.tragetTile` _tile)
      (else
        (bind _tile_2 (`/Game/Control/BP_Path.getNext` _value))
        (set `self.tragetTile` _tile_2))))
  (if (< _returnvalue_z _returnvalue_z_2)
    (set `self.targetPosition` (`KismetMathLibrary.MakeVector` _returnvalue_x _returnvalue_y _returnvalue_z_2))
    (`self.EventToMove`)
    (elif (`KismetMathLibrary.BooleanNAND` (== _returnvalue_x _returnvalue_x_2) (== _returnvalue_y _returnvalue_y_2))
      (set `self.targetPosition` (`KismetMathLibrary.MakeVector` _returnvalue_x_2 _returnvalue_y_2 _returnvalue_z))
      (`self.EventToMove`)
      (else
        (set `self.targetPosition` (`KismetMathLibrary.MakeVector` _returnvalue_x_2 _returnvalue_y_2 _returnvalue_z_2))
        (`self.EventToMove`)))))

(fn `dismiss`
  (`self.unmarkRaech`)
  (`KismetArrayLibrary.Array_RemoveItem` (`/Game/Hex/BP_HexTile.Units` (`self.currentTile`)) self)
  (`KismetArrayLibrary.Array_RemoveItem` (`/Game/Control/Factions/BPFaction.Owned` (`self.faction`)) self)
  (`self.K2_DestroyActor`))

(fn `makeStep`
  (params (deltaTime :type "Float (double-precision)"))
  (`self.K2_SetActorLocation` (`KismetMathLibrary.VInterpTo_Constant` (`self.K2_GetActorLocation`) (`self.targetPosition`) deltaTime (`self.MOVE_SPEED`))))

(fn `markReach`
  (`self.unmarkRaech`)
  (`BlueprintMapLibrary.Map_Clear` (`self.reachMap`))
  (`/Game/Hex/BP_HexTile.markReachSelf` (`self.currentTile`) self (`self.movePt`) 0.0 (`|MakeArray`)))

(fn `moveCurrentTile`
  (params (newCurrent :type "/Game/Hex/BP_HexTile Object Reference"))
  (`KismetArrayLibrary.Array_RemoveItem` (`/Game/Hex/BP_HexTile.Units` (`self.currentTile`)) self)
  (bind _output_get (set `self.currentTile` newCurrent))
  (`KismetArrayLibrary.Array_Add` (`/Game/Hex/BP_HexTile.Units` _output_get) self))

(fn `moveTo`
  (bind _value (`BlueprintMapLibrary.Map_Find` (`self.reachMap`) (`self.finishTile`)))
  (if (== (`self.K2_GetActorLocation`) (`self.K2_GetActorLocation` (`self.currentTile`)))
    (if (`/Game/Control/BP_Path.enemyPresent` _value)
      (bind _enemypresent (`self.attackEnemy`))
      (set `/Game/Control/BP_Path.attacked` true _value)
      (if _enemypresent
        (bind _tile (`/Game/Control/BP_Path.getPrev` _value))
        (bind _output_get (set `self.finishTile` _tile))
        (`self.markReach`)
        (`self.navigateTo` _output_get)
        (else
          (set `self.moving` false :!label _label)
          (cast `/Game/Control/Factions/BPAiFaction` (`self.faction`)
            (:`CastFailed`
              (bind _asbp_instance (cast `/Game/Control/BP_Instance` (`GameplayStatics.GetGameInstance`)))
              (`self.markReach`)
              (set `/Game/Control/BP_Instance.SelectedTile` (`self.currentTile`) _asbp_instance)
              (`/Game/Control/BP_Instance.getHUD` _asbp_instance)))))
      (else
        (goto _label)))
    (else
      (`self.choosePosition`))))

(fn `nameUnit`
  (params (order :type Integer))
  (set `self.name` (`KismetStringLibrary.Concat_StrStr` "unit " (`KismetStringLibrary.Conv_IntToString` order))))

(fn `navigateTo`
  (params (tile :type "/Game/Hex/BP_HexTile Object Reference"))
  (set `self.moving` true)
  (`self.moveCurrentTile` tile)
  (bind _output_get (set `self.finishTile` tile))
  (bind _value (`BlueprintMapLibrary.Map_Find` (`self.reachMap`) _output_get))
  (set `self.movePt` (- (`self.movePt`) (`/Game/Control/BP_Path.cost` _value)))
  (bind _tile (`/Game/Control/BP_Path.getNext` _value))
  (set `self.tragetTile` _tile)
  (`self.moveTo`))

(fn `nearTarget`
  (returns (ret :type Boolean))
  (return (<= (`KismetMathLibrary.Vector_Distance` (`self.K2_GetActorLocation`) (`self.targetPosition`)) 0.5)))

(fn `select`
  (bind _asbp_instance (cast `/Game/Control/BP_Instance` (`GameplayStatics.GetGameInstance`)))
  (`/Game/Control/BP_Instance.clickUnit` _asbp_instance self)
  (if (`KismetArrayLibrary.Array_Contains` (`/Game/Control/Factions/BPFaction.Owned` (`|GetArrayItem` (`/Game/Control/BP_Instance.Factions` _asbp_instance) (`/Game/Control/BP_Instance.factionInd` _asbp_instance))) self)
    (`self.markReach`)))

(fn `unmarkRaech`
  (bind _keys (`BlueprintMapLibrary.Map_Keys` (`self.reachMap`)))
  (for _array_element _keys
    (`/Game/Hex/BP_HexTile.unsetMarker` _array_element)))

(fn `UserConstructionScript`
  (bind _color (`self.color`))
  (`parent.UserConstructionScript`)
  (`PrimitiveComponent.SetMaterial` (`self.Cube`) 0 _color)
  (`PrimitiveComponent.SetMaterial` (`self.Cone`) 0 _color)
  (`/Game/Hex/BP_HexTile.addUnit` (`self.currentTile`) self))
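; BP_settler is a placeable settler unit that can found a holding on the tile it occupies.
; On BeginPlay it runs the parent logic, then applies its Color material to the second material slot of the Settler component.
; Settle checks that the current tile has no valid holding, has the Faction spawn a BP_Holding there, and registers it with the tile.
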(event `self.ReceiveBeginPlay`
  (`parent.ReceiveBeginPlay`)
  (`PrimitiveComponent.SetMaterial` (`self.settler`) 1 (`self.color`)))

(fn `settle`
  (bind _currenttile (`self.currentTile`))
  (`/Engine/EditorBlueprintResources/StandardMacros.IsValid` (`/Game/Hex/BP_HexTile.holding` _currenttile)
    (:`Is Not Valid`
      (bind _newparam (`/Game/Control/Factions/BPFaction.spawnPlaceble` (`self.faction`) _currenttile "/Game/Placeable/BP_Holding.BP_Holding_C"))
      (bind _asbp_holding (cast `/Game/Placeable/BP_Holding` _newparam))
      (`/Game/Hex/BP_HexTile.addHolding` _currenttile _asbp_holding))))

(fn `UserConstructionScript`
  (`parent.UserConstructionScript`))
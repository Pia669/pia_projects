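; BP_Placable is a placeable actor on a tile in a turn-based game, with combat stats, visibility and production.
; NewTurn fires the empty EventNewTurn hook, then returns Production.
; Attacked applies attack minus defence, then either counterattacks at half Attack or destroys the actor, first removing it from CurrentTile if it is a BP_Unit.
; UncoverVisible and HideVisible pass Visibility to CurrentTile to reveal or hide tiles.
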(event `EventNewTurn`)

(fn `attacked`
  (params (attacker :type "/Game/Placeable/BP_Placable Object Reference"))
  (returns (survive :type Boolean))
  (bind _output_get (set `self.health` (- (`self.health`) (- (`/Game/Placeable/BP_Placable.attack` attacker) (`self.defence`)))))
  (if (> _output_get 0.0)
    (set `/Game/Placeable/BP_Placable.health` (- (`/Game/Placeable/BP_Placable.health` attacker) (- (/ (`self.attack`) 2.0) (`/Game/Placeable/BP_Placable.defence` attacker))) attacker)
    (return true)
    (else
      (bind _asbp_unit (cast `/Game/Placeable/BP_Unit` self)
        (:`then`
          (`/Game/Hex/BP_HexTile.removeUnit` (`self.currentTile`) _asbp_unit))
        (:`CastFailed`
          _))
      (`self.K2_DestroyActor`)
      (return false))))

(fn `hideVisible`
  (`/Game/Hex/BP_HexTile.hide` (`self.currentTile`) (`self.visibility`)))

(fn `newTurn`
  (returns (production :type "Array of Float (double-precision)"))
  (`self.EventNewTurn`)
  (return (`self.production`)))

(fn `uncoverVisible`
  (`/Game/Hex/BP_HexTile.uncover` (`self.currentTile`) (`self.visibility`)))

(fn `UserConstructionScript`)
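; BP_Holding is a placeable, faction-owned holding on a tile map that trains units in a turn-based game.
; On construction it applies its color material and registers with its current tile.
; Each new turn it spawns the first queued unit through BP_Instance on that tile, then dequeues it.
; IsInDanger recursively checks for enemies at depth two, which covers only its own tile and immediate neighbours.
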(event `self.ReceiveBeginPlay`
  (`parent.ReceiveBeginPlay`))

(event `self.EventNewTurn`
  (bind _prodque (`self.prodQue`))
  (bind _faction (`self.faction`))
  (`parent.EventNewTurn`)
  (if (`KismetArrayLibrary.Array_IsNotEmpty` _prodque)
    (bind _asbp_instance (cast `/Game/Control/BP_Instance` (`GameplayStatics.GetGameInstance`)))
    (`/Game/Control/BP_Instance.spawnUnit` _asbp_instance (`self.currentTile`) (`/Game/Control/Factions/BPFaction.Color` _faction) _faction (`|GetArrayItem` _prodque))
    (`KismetArrayLibrary.Array_Remove` _prodque)))

(fn `isInDanger`
  (returns (ret :type Boolean))
  (bind _isindanger (`self.isInDangerTile` 2 (`self.currentTile`)))
  (return _isindanger))

(fn `isInDangerTile`
  (params (dist :type Integer) (tile :type "/Game/Hex/BP_HexTile Object Reference"))
  (returns (isInDanger :type Boolean))
  (if (== dist 0)
    (return false)
    (else
      (bind _present (`/Game/Hex/BP_HexTile.enemyPresent` tile self))
      (if _present
        (return true)
        (else
          (bind _tiles (`/Game/Hex/BP_HexTile.getNeigbours` tile))
          (for _array_element _tiles
            (bind _isindanger (`self.isInDangerTile` (- (`local.dist`) 1) _array_element))
            (if _isindanger
              (return true)))
          (return false))))))

(fn `nameHolding`
  (params (order :type Integer))
  (set `self.name` (`KismetStringLibrary.Concat_StrStr` "holding " (`KismetStringLibrary.Conv_IntToString` order))))

(fn `UserConstructionScript`
  (`parent.UserConstructionScript`)
  (`PrimitiveComponent.SetMaterial` (`self.body`) 0 (`self.color`))
  (`/Game/Hex/BP_HexTile.addHolding` (`self.currentTile`) self))
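; Hex map generator actor that spawns a grid of BP_HexTile actors with procedural height, temperature and precipitation.
; Three randomly seeded Perlin noise maps supply variation, with cosine latitude curves shaping temperature and precipitation by row.
; GenerateNewMap stores tiles for row/column lookup, spawns a plane and four borders, then picks random faction starts via BP_Instance, excluding sea, deep sea and ice biomes.
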(event `self.ReceiveBeginPlay`)

(fn `calcPercipitation`
  (params (row :type Integer) (col :type Integer))
  (returns (percipitation :type Integer))
  (bind _perc_vria (`self.PERC_VRIA`))
  (bind _max_perc (`self.MAX_PERC`))
  (bind _returnvalue (/ (`self.N_ROWS`) (`KismetMathLibrary.GetPI`)))
  (bind _ret (`self.rowToFunc` row _returnvalue))
  (bind _ret_2 (`self.rowToFunc` row (/ _returnvalue 3.0)))
  (bind _value (`self.getNoiseValue` (`self.PersepitationNoise`) row col))
  (bind _scaledvalue (`self.scaleRange` _value -0.8 0.8 (/ _max_perc (* _perc_vria -1)) (/ _max_perc _perc_vria)))
  (return (`KismetMathLibrary.FTrunc` (`KismetMathLibrary.FMax` (+ (* (/ _ret 2.0) (* _ret_2 3.0) (`self.MAX_PERC`)) _scaledvalue)))))

(fn `calcTemperature`
  (params (row :type Integer) (col :type Integer))
  (returns (temperature :type "Float (double-precision)"))
  (bind _min_temp (`self.MIN_TEMP`))
  (bind _returnvalue (/ (+ (`self.MAX_TEMP`) (`KismetMathLibrary.Abs` _min_temp)) 2.0))
  (bind _value (`self.getNoiseValue` (`self.TemperaturNoise`) row col))
  (bind _scaledvalue (`self.scaleRange` _value -0.8 0.8 (/ (`self.MIN_TEMP`) 5.0) (/ (`self.MAX_TEMP`) 5.0)))
  (return (+ (+ (+ _min_temp _returnvalue) (* _returnvalue (`KismetMathLibrary.Cos` (/ row (/ (`self.N_ROWS`) (`KismetMathLibrary.GetPI`)))))) _scaledvalue)))

(fn `calcTileProps`
  (params (row :type Integer) (col :type Integer))
  (returns (height :type "Float (double-precision)") (temperature :type "Float (double-precision)") (persepitation :type Integer))
  (bind _percipitation (`self.calcPercipitation` row col))
  (bind _temperature (`self.calcTemperature` row col))
  (bind _height (`self.clacHeight` row col))
  (return _height _temperature _percipitation))

(fn `checkLocation`
  (params (tile :type "/Game/Hex/BP_HexTile Object Reference"))
  (returns (suitable :type Boolean))
  (bind _biome (`/Game/Hex/BP_HexTile.Biome` tile))
  (return (not (or (`GameplayStatics.ObjectIsA` _biome "/Game/Hex/Biomes/BP_DeepSeaBiome.BP_DeepSeaBiome_C") (`GameplayStatics.ObjectIsA` _biome "/Game/Hex/Biomes/BP_SeaBiome.BP_SeaBiome_C") (`GameplayStatics.ObjectIsA` _biome "/Game/Hex/Biomes/BP_IceBiome.BP_IceBiome_C")))))

(fn `chooseStartLocations`
  (locals (tile :type "/Game/Hex/BP_HexTile Object Reference"))
  (bind _tiles (`self.Tiles`))
  (bind _asbp_instance (cast `/Game/Control/BP_Instance` (`GameplayStatics.GetGameInstance`)))
  (while (< (`KismetArrayLibrary.Array_Length` (`/Game/Control/BP_Instance.Factions` _asbp_instance)) (`/Game/Control/BP_Instance.N_FACTIONS` _asbp_instance))
    (bind _output_get (set `local.tile` (`|GetArrayItem` _tiles (`KismetMathLibrary.RandomInteger` (`KismetArrayLibrary.Array_Length` _tiles)))))
    (bind _suitable (`self.checkLocation` _output_get))
    (if _suitable
      (`/Game/Control/BP_Instance.factStartLocation` _asbp_instance _output_get))))

(fn `clacHeight`
  (params (row :type Integer) (col :type Integer))
  (returns (height :type "Float (double-precision)"))
  (bind _value (`self.getNoiseValue` (`self.HeightNoise`) row col))
  (bind _scaledvalue (`self.scaleRange` _value -0.8 0.8 0.0 (`self.MAX_HEIGHT`)))
  (return (- _scaledvalue (`self.SEA_LEVEL`))))

(fn `generateNewMap`
  (bind _n_cols (`self.N_COLS`))
  (bind _tiles (`self.Tiles`))
  (bind _n_rows (`self.N_ROWS`))
  (`self.setupNoiseMaps`)
  (for _index (range (* -1 _n_rows) (+ _n_rows 1))
    (for _index_2 (range (* -1 _n_cols) (+ _n_cols 1))
      (bind (_height _temperature _persepitation) (`self.calcTileProps` _index _index_2))
      (bind _returnvalue (`|SpawnActorFromClass` "/Game/Hex/BP_HexTile.BP_HexTile_C" (`self.GetTransform`) "Undefined" "MultiplyWithRoot" null self _index _index_2 _height _temperature _persepitation null))
      (`KismetArrayLibrary.Array_Add` (`self.Tiles`) _returnvalue)))
  (`self.makeMapBorder` (`|GetArrayItem` _tiles (- (`KismetArrayLibrary.Array_Length` _tiles) 1)) (`|GetArrayItem` _tiles))
  (`self.chooseStartLocations`))

(fn `getNoiseValue`
  (params (noise :type "FastNoiseWrapper Object Reference") (row :type Integer) (col :type Integer))
  (returns (value :type "Float (double-precision)"))
  (return (`FastNoiseWrapper.GetNoise2D` noise (`KismetMathLibrary.Conv_IntToDouble` (* row 10)) (`KismetMathLibrary.Conv_IntToDouble` (* col 10)))))

(fn `getTile`
  (params (row :type Integer) (col :type Integer))
  (returns (tile :type "/Game/Hex/BP_HexTile Object Reference"))
  (if (and (<= (`KismetMathLibrary.Abs_Int` row) (`self.N_ROWS`)) (<= (`KismetMathLibrary.Abs_Int` col) (`self.N_COLS`)))
    (return (`|GetArrayItem` (`self.Tiles`) (+ (* (+ (* (`self.N_COLS`) 2) 1) (+ (`self.N_ROWS`) row)) (+ col (`self.N_COLS`)))))))

(fn `makeMapBorder`
  (params (topLeft :type "/Game/Hex/BP_HexTile Object Reference") (bottomRight :type "/Game/Hex/BP_HexTile Object Reference"))
  (bind (_returnvalue_x _returnvalue_y) (`KismetMathLibrary.BreakVector` (`self.K2_GetActorLocation` bottomRight)))
  (bind (_returnvalue_x_2 _returnvalue_y_2) (`KismetMathLibrary.BreakVector` (`self.K2_GetActorLocation` topLeft)))
  (bind (_scalex _scaley) (`self.planeScale` _returnvalue_x _returnvalue_y))
  (`|SpawnActorFromClass` "/Game/Hex/Map/BP_Plane.BP_Plane_C" (`KismetMathLibrary.MakeTransform` (0.0 0.0 0.0) (struct) (`KismetMathLibrary.MakeVector` _scalex _scaley 1.0)) "Undefined" "MultiplyWithRoot" null null)
  (`|SpawnActorFromClass` "/Game/Hex/Map/BP_Border.BP_Border_C" (`KismetMathLibrary.MakeTransform` (`KismetMathLibrary.MakeVector` (+ _returnvalue_x_2 100.0)) (struct) (`KismetMathLibrary.MakeVector` 1.0 (+ (`self.tileDisToScale` _returnvalue_y_2) 1.0) 1.0)) "Undefined" "MultiplyWithRoot" null null)
  (`|SpawnActorFromClass` "/Game/Hex/Map/BP_Border.BP_Border_C" (`KismetMathLibrary.MakeTransform` (`KismetMathLibrary.MakeVector` (- _returnvalue_x 100.0)) (struct) (`KismetMathLibrary.MakeVector` 1.0 (+ (`self.tileDisToScale` _returnvalue_y) 1.0) 1.0)) "Undefined" "MultiplyWithRoot" null null)
  (`|SpawnActorFromClass` "/Game/Hex/Map/BP_Border.BP_Border_C" (`KismetMathLibrary.MakeTransform` (`KismetMathLibrary.MakeVector` 0.0 (+ _returnvalue_y_2 100.0)) (struct) (`KismetMathLibrary.MakeVector` (- (`self.tileDisToScale` _returnvalue_x_2) 1.0) 1.0 1.0)) "Undefined" "MultiplyWithRoot" null null)
  (`|SpawnActorFromClass` "/Game/Hex/Map/BP_Border.BP_Border_C" (`KismetMathLibrary.MakeTransform` (`KismetMathLibrary.MakeVector` 0.0 (- _returnvalue_y 100.0)) (struct) (`KismetMathLibrary.MakeVector` (- (`self.tileDisToScale` _returnvalue_x) 1.0) 1.0 1.0)) "Undefined" "MultiplyWithRoot" null null))

(fn `rowToFunc`
  (params (row :type Integer) (div :type "Float (double-precision)"))
  (returns (ret :type "Float (double-precision)"))
  (return (+ (/ (`KismetMathLibrary.Cos` (/ row div)) 2.0) 0.5)))

(fn `scaleRange`
  (params (valueToScale :type "Float (double-precision)") (orgMin :type "Float (double-precision)") (orgMax :type "Float (double-precision)") (newMin :type "Float (double-precision)") (newMax :type "Float (double-precision)"))
  (returns (scaledValue :type "Float (double-precision)"))
  (return (+ (/ (* (- valueToScale orgMin) (- newMax newMin)) (- orgMax orgMin)) newMin)))

(fn `setupNoiseMaps`
  (bind _returnvalue (`|GenericCreateObject` "/Script/FastNoiseGenerator.FastNoiseWrapper"))
  (bind _output_get (set `self.HeightNoise` _returnvalue))
  (`FastNoiseWrapper.SetupFastNoise` _output_get "Perlin" (`KismetMathLibrary.RandomIntegerInRange` -10000 10000) 0.01 "Quintic" "FBM" 3 2.0 0.5 0.45 "Euclidean" "CellValue")
  (bind _returnvalue_2 (`|GenericCreateObject` "/Script/FastNoiseGenerator.FastNoiseWrapper"))
  (bind _output_get_2 (set `self.TemperaturNoise` _returnvalue_2))
  (`FastNoiseWrapper.SetupFastNoise` _output_get_2 "Perlin" (`KismetMathLibrary.RandomIntegerInRange` -10000 10000) 0.01 "Quintic" "FBM" 3 2.0 0.5 0.45 "Euclidean" "CellValue")
  (bind _returnvalue_3 (`|GenericCreateObject` "/Script/FastNoiseGenerator.FastNoiseWrapper"))
  (bind _output_get_3 (set `self.PersepitationNoise` _returnvalue_3))
  (`FastNoiseWrapper.SetupFastNoise` _output_get_3 "Perlin" (`KismetMathLibrary.RandomIntegerInRange` -10000 10000) 0.01 "Quintic" "FBM" 3 2.0 0.5 0.45 "Euclidean" "CellValue"))

(fn `UserConstructionScript`)